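; Racing game mode that runs a countdown, starts a timed race and declares a win or loss.
; On BeginPlay it binds to the crossed event of every finish-line checkpoint, then starts the countdown.
; When the delay ends, a one-shot timer triggers a loss on expiry, while the win event clears it.
; Countdown, start and result feedback are only debug print strings.
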(event Custom|Game%20Start
  (Development|PrintString "The game has started")
  (bind _returnvalue (Utilities|Time|SetTimerbyEvent (delegate Custom|Lose_OutOfTIme) (Variables|Default|GetStartTimerDuration)))
  (Variables|Default|SetTimeRemainignTimer _returnvalue))

(event Custom|Game%20Finish
  (params (Win :type Boolean))
  (Development|PrintString (Utilities|String|SelectString "You Win!" "You Lost" Win)))

(event Custom|Start%20Countdown
  (Development|PrintString "Start Countdown")
  (Utilities|FlowControl|Delay (Variables|Default|GetStartCountownDuration))
  (CallFunction|GameStart))

(event Custom|Lose_OutOfTIme
  (CallFunction|GameFinish false))

(event Custom|Win_CrossTheFinishLine
  (Utilities|Time|ClearandInvalidateTimerbyHandle (Variables|Default|GetTimeRemainignTimer))
  (CallFunction|GameFinish true))

(event EventBeginPlay
  (Utilities|FlowControl|Sequence
    (:then_0
      (bind _outactors (Actor|GetAllActorsOfClass "/Game/RacingGame/Checkpoints/BP_Chekpoint.BP_Chekpoint_C"))
      (for _array_element _outactors
        (if (Variables|/Game/RacingGame/Checkpoints/BP_Chekpoint.BP_Chekpoint_C|GetIsFinishLine _array_element)
          (EventDispatchers|BindEventtoOnCheckpointCrossed _array_element (EventDispatchers|CreateEvent :!event Custom|Win_CrossTheFinishLine)))))
    (:then_1
      (CallFunction|StartCountdown))))

(fn ConstructionScript)